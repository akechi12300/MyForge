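; BP_Cube is a cube block actor that exposes six connection points (接続点).
; Its construction script calls the parent's, then clears the 接続点 array and refills it with 接続点01 through 接続点06.
; The event graph has no active logic: Tick is empty, and an unconnected forward line trace with debug drawing never runs.
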(event EventBeginPlay
  (|CallParentFunction) ; このノードは無効になっているため呼び出せません。\n機能をビルドするにはピンをドラッグしてください。
)

(event Collision|EventActorBeginOverlap
  (params (OtherActor :type Actor%20Object%20Reference))
  (|CallParentFunction OtherActor) ; このノードは無効になっているため呼び出せません。\n機能をビルドするにはピンをドラッグしてください。
)

(event EventTick
  (params (DeltaSeconds :type Float%20%28single-precision%29)))

(fn ConstructionScript
  (bind _接続点 (Variables|Default|Get接続点))
  (|CallParentFunction)
  (Utilities|Array|Clear _接続点)
  (Utilities|Array|Add _接続点 (Variables|Default|Get接続点01))
  (Utilities|Array|Add _接続点 (Variables|Default|Get接続点02))
  (Utilities|Array|Add _接続点 (Variables|Default|Get接続点03))
  (Utilities|Array|Add _接続点 (Variables|Default|Get接続点04))
  (Utilities|Array|Add _接続点 (Variables|Default|Get接続点05))
  (Utilities|Array|Add _接続点 (Variables|Default|Get接続点06)))