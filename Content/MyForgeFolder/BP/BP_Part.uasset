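; BP_Part is a connectable part that starts as its own group and finds connection candidates for a held group.
; 最短距離方式 box-traces around each held part, alternates closest-point-on-collision queries to converge on nearest surface points, and keeps the closest pair and target.
; 接続候補を取得テスト prints that result.
; Connection-point trace approaches are left unwired, and the group-bounds function is empty.
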(event Collision|EventActorBeginOverlap
  (params (OtherActor :type Actor%20Object%20Reference)))

(event EventTick
  (params (DeltaSeconds :type Float%20%28single-precision%29)))

(event EventBeginPlay
  (|CallParentFunction)
  (Utilities|Array|Clear (Variables|Default|Getパーツグループ))
  (Utilities|Array|Add (Variables|Default|Getパーツグループ) self))

(fn ConstructionScript)

(fn 接続候補を取得テスト
  (params (掴み中パーツ :type BP%20Part%20Object%20Reference))
  (bind (_newparam _newparam1 _newparam2) (CallFunction|最短距離方式 掴み中パーツ))
  (Development|PrintString (Utilities|String|ToString(Vector) _newparam) true true "(R=0.000000,G=0.660000,B=1.000000,A=1.000000)" 0.0)
  (Development|PrintString (Utilities|String|ToString(Vector) _newparam1) true true "(R=0.000000,G=0.660000,B=1.000000,A=1.000000)" 0.0)
  (Development|PrintString (Utilities|GetDisplayName _newparam2) true true "(R=0.000000,G=0.660000,B=1.000000,A=1.000000)" 0.0))

(fn 最短距離方式
  (params (掴み中パーツ :type BP%20Part%20Object%20Reference))
  (bind _パーツグループ (Variables|BP_Part_C|Getパーツグループ 掴み中パーツ))
  (LocalVariables|Setパーツ単体の最短距離点Ａ "0, 0, 0")
  (LocalVariables|Setパーツ単体の最短距離点Ｂ "0, 0, 0")
  (LocalVariables|Setベストな距離 999999.0)
  (for _array_element _パーツグループ
    (bind _outhits (Class|KismetSystemLibrary|BoxTraceMulti (.Origin (Collision|GetActorBounds _array_element true false)) (.Origin (Collision|GetActorBounds _array_element true false)) (* (.BoxExtent (Collision|GetActorBounds _array_element true false)) 2.0) "0, 0, 0" "TraceTypeQuery4" true _パーツグループ "ForOneFrame" false))
    (for _array_element_2 _outhits
      (LocalVariables|SetポイントＡ (Physics|GetCenterOfMass (Variables|/Game/MyForgeFolder/BP/BP_Connectable.BP_Connectable_C|Getルートメッシュ _array_element) "None"))
      (for _index (range 0 15)
        (bind _output_get (LocalVariables|SetポイントＢ (.OutPointOnBody (Collision|GetClosestPointonCollision (.HitComponent (Collision|BreakHitResult _array_element_2)) (LocalVariables|GetポイントＡ) "None"))))
        (LocalVariables|SetポイントＡ (.OutPointOnBody (Collision|GetClosestPointonCollision (Variables|/Game/MyForgeFolder/BP/BP_Connectable.BP_Connectable_C|Getルートメッシュ _array_element) _output_get "None"))))
      (if (<= (Math|Vector|Distance(Vector) (LocalVariables|GetポイントＡ) (LocalVariables|GetポイントＢ)) (LocalVariables|Getベストな距離))
        (LocalVariables|Setベストな距離 (Math|Vector|Distance(Vector) (LocalVariables|GetポイントＡ) (LocalVariables|GetポイントＢ)))
        (LocalVariables|Setパーツ単体の最短距離点Ａ (LocalVariables|GetポイントＡ))
        (LocalVariables|Setパーツ単体の最短距離点Ｂ (LocalVariables|GetポイントＢ))
        (bind _asbp_connectable (Utilities|Casting|CastToBP_Connectable (.HitActor (Collision|BreakHitResult _array_element_2))))
        (bind _output_get_2 (LocalVariables|Set接続相手Connectable _asbp_connectable))
        (bind _asbp_part (Utilities|Casting|CastToBP_Part _output_get_2))
        (LocalVariables|Set接続相手Part _asbp_part))))
  (Rendering|Debug|DrawDebugPoint (LocalVariables|Getパーツ単体の最短距離点Ａ) 2e+01 "(R=1.000000,G=0.095705,B=0.000000,A=1.000000)" 0.0)
  (Rendering|Debug|DrawDebugPoint (LocalVariables|Getパーツ単体の最短距離点Ｂ) 2e+01 "(R=0.000000,G=0.074790,B=1.000000,A=1.000000)" 0.0)
  (return (LocalVariables|Getパーツ単体の最短距離点Ａ) (LocalVariables|Getパーツ単体の最短距離点Ｂ) (LocalVariables|Get接続相手Connectable)))

(fn パーツ群のBoundsを求める関数)